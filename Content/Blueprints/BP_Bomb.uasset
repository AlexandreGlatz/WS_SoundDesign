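; Bomb actor that plays a bomb sound and muffles game audio when the third-person character enters its sphere.
; The overlap spawns an attached sound and watches its MetaSound "BombExploded" output, so the audio itself times when the muffled sound mix is pushed.
; The mix is never popped, overlaps can retrigger, and the audio-finished callback only prints a debug string.
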(event `self.Sphere.OnComponentBeginOverlap`
  (params (OverlappedComponent :type "PrimitiveComponent Object Reference") (OtherActor :type "Actor Object Reference") (OtherComp :type "PrimitiveComponent Object Reference") (OtherBodyIndex :type Integer) (bFromSweep :type Boolean) (SweepResult :type "HitResult Structure (by ref)"))
  (cast `/Game/ThirdPerson/Blueprints/BP_ThirdPersonCharacter` OtherActor)
  (bind _returnvalue (`GameplayStatics.SpawnSoundAttached` "/Game/Audio/MetaSound/AMB/SFX_Bomb.SFX_Bomb" (`self.Sphere`) "None" (0.0 0.0 0.0) (struct) "KeepRelativeOffset" false 1.0 1.0 0.0 null null))
  (`AudioComponent.Play` _returnvalue 0.0)
  (add `AudioComponent.OnAudioFinished` _returnvalue (delegate `CustomEvent`))
  (`MetaSoundOutputSubsystem.WatchOutput` (subsystem `MetaSoundOutputSubsystem`) _returnvalue "BombExploded" (delegate `Audio_BombEffect`) "None" "None"))

(event `CustomEvent`
  (`KismetSystemLibrary.PrintString` "Hello"))

(event `Audio_BombEffect`
  (params (OutputName :type Name) (Output :type "MetaSoundOutput Structure (by ref)"))
  (`GameplayStatics.PushSoundMixModifier` "/Game/Audio/MetaSound/AMB/SMMMuffled.SMMMuffled"))

(fn `UserConstructionScript`)